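; Sliding door Blueprint that moves the actor vertically between its start location and an offset set by DoorHeight.
; On BeginPlay it stores the start location and, if StartOpen is set, negates DoorHeight to invert the slide direction.
; The toggleDoor event plays or reverses a timeline that scales the Z offset, and SwitchDirection flips when each run finishes.
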(event `self.ReceiveBeginPlay`
  ;[1 1 1] Check to see if door starts open
  (set `self.startLoc` (`self.K2_GetActorLocation`))
  (if (`self.StartOpen`)
    (`self.toggleDoorOpen`)))

(event `self.ReceiveTick`
  (params (DeltaSeconds :type "Float (single-precision)")))

(event `toggleDoorOpen`
  ;[1 1 1] Switch Door between opening/closing
  (set `self.DoorHeight` (* (`self.DoorHeight`) -1.0)))

(event `toggleDoor`
  ;[1 1 1] Open/Close Door
  (if (`self.switchDirection`)
    (bind (_direction _newtrack_1) (`Timeline|toggleDoorTL` :!via `Reverse` :!label _label)
      (:`Update`
        (`self.K2_SetActorLocation` (+ (`KismetMathLibrary.MakeVector` 0.0 0.0 (* _newtrack_1 (`self.DoorHeight`))) (`self.startLoc`))))
      (:`Finished`
        (if (`self.switchDirection`)
          (set `self.switchDirection` false)
          (else
            (set `self.switchDirection` true)))))
    (else
      (goto _label))))

(fn `UserConstructionScript`)