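; ConveyorBP is a conveyor actor that carries player platforms along its forward direction and can optionally act as a cannon.
; Each tick it offsets every PlayerPlatformBP overlapping its Box by a per-instance Speed, without sweeping.
; With IsCannon set, a platform leaving the overlap gets its physics velocity replaced by a forward launch, with an explosion sound.
; The construction script counter-scales the Arrow to keep it readable in the editor.
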(event `self.ReceiveActorEndOverlap`
  (params (OtherActor :type "Actor Object Reference"))
  (if (`self.isCannon`)
    (if (== (`GameplayStatics.GetObjectClass` OtherActor) "/Game/Blueprints/PlayerPlatformBP.PlayerPlatformBP_C")
      (bind _asplayer_platform_bp (cast `/Game/Blueprints/PlayerPlatformBP` OtherActor))
      (`PrimitiveComponent.SetPhysicsLinearVelocity` (`StaticMeshActor.StaticMeshComponent` _asplayer_platform_bp) (* (`KismetMathLibrary.GetForwardVector` (`self.K2_GetActorRotation`)) (`self.Velocity`)) false "None")
      (`GameplayStatics.PlaySoundAtLocation` "/Game/audio/StarterContent/Audio/Explosion01.Explosion01" (`self.K2_GetActorLocation` _asplayer_platform_bp)))))

(event `self.ReceiveTick`
  (params (DeltaSeconds :type "Float (single-precision)"))
  (for _array_element (`PrimitiveComponent.GetOverlappingActors` (`self.Box`) "/Game/Blueprints/PlayerPlatformBP.PlayerPlatformBP_C")
    (`self.K2_AddActorWorldOffset` _array_element (* (`KismetMathLibrary.GetForwardVector` (`self.K2_GetActorRotation`)) (* DeltaSeconds (`self.Speed`))) false false)))

(fn `UserConstructionScript`
  (`SceneComponent.SetRelativeScale3D` (`self.Arrow`) (/ (2.0 2.0 2.0) (`self.GetActorScale3D`))) ; keeps editor arrow from \ngetting too large for the collider
)