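; Pressure plate actor that sinks when a PlayerPlatformBP actor overlaps it and rises back when the overlap ends.
; BeginPlay caches the mesh's world location, and overlap events ease it between that position and a lowered one via MoveComponentTo, passed as relative location.
; Both press and release pulse the Trigger flag true briefly, with a delay so the door can catch it.
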(event `self.ReceiveBeginPlay`
  (set `self.Original Location` (`SceneComponent.K2_GetComponentLocation` (`self.StaticMeshComponent`))))

(event `self.ReceiveActorBeginOverlap`
  (params (OtherActor :type "Actor Object Reference"))
  (if (== (`GameplayStatics.GetObjectClass` OtherActor) "/Game/Blueprints/PlayerPlatformBP.PlayerPlatformBP_C")
    (`self.Send trigger message`)
    (set `self.destination` (- (`self.Original Location`) (0.0 0.0 20.0)))
    (`KismetSystemLibrary.MoveComponentTo` (`self.StaticMeshComponent`) (`self.destination`) (struct) true true :!label _label)))

(event `self.ReceiveActorEndOverlap`
  (params (OtherActor :type "Actor Object Reference"))
  (if (== (`GameplayStatics.GetObjectClass` (stale `self.ReceiveActorBeginOverlap` OtherActor)) "/Game/Blueprints/PlayerPlatformBP.PlayerPlatformBP_C")
    (`self.Send trigger message`)
    (set `self.destination` (`self.Original Location`))
    (goto _label)))

(event `Send trigger message`
  (set `self.Trigger` true)
  (`KismetSystemLibrary.Delay` 0.2) ; need delay or the door \ndoesnt catch trigger being on
  (set `self.Trigger` false))

(fn `UserConstructionScript`)